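; BP_RadiationField is a map boundary actor that keeps the player inside a safe sphere, framed as dangerous surface radiation.
; When BP_FirstPersonCharacter leaves the sphere, it saves the exit location and starts a short timer, which re-entering cancels.
; If the timer expires, it moves the player back to the saved location and has the ARIS AI brain deliver a scripted German radiation warning.
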(event OnComponentEndOverlap(Sphere)
  (params (OverlappedComponent :type Primitive%20Component%20Object%20Reference) (OtherActor :type Actor%20Object%20Reference) (OtherComp :type Primitive%20Component%20Object%20Reference) (OtherBodyIndex :type Integer))
  (Utilities|Casting|CastToBP_FirstPersonCharacter OtherActor)
  (Development|PrintString "Danger")
  (Variables|Default|SetLocation (Transformation|GetActorLocation (CallFunction|GetDirectPlayerController)))
  (bind _returnvalue (Utilities|Time|SetTimerbyFunctionName 0 "TeleportPlayerBackInside" 6.0))
  (Variables|Default|SetDestructionTimer _returnvalue))

(event OnComponentBeginOverlap(Sphere)
  (params (OverlappedComponent :type Primitive%20Component%20Object%20Reference) (OtherActor :type Actor%20Object%20Reference) (OtherComp :type Primitive%20Component%20Object%20Reference) (OtherBodyIndex :type Integer) (bFromSweep :type Boolean) (SweepResult :type Hit%20Result%20Structure%20%28by%20ref%29))
  (Utilities|Casting|CastToBP_FirstPersonCharacter OtherActor)
  (Development|PrintString "Danger Averted")
  (Utilities|Time|ClearandInvalidateTimerbyHandle (Variables|Default|GetDestructionTimer)))

(event Custom|TeleportPlayerBackInside
  (Development|PrintString "Died")
  (Transformation|SetActorLocation (CallFunction|GetDirectPlayerController) (Variables|Default|GetLocation) false false)
  (Default|ProcessDialogue (.AC_AIBrain (CallFunction|GetDirectARIS)) true "Operator, die Strahlung auf der Oberfläche ist gefährlich, geht nicht zu weit raus."))

(event EventBeginPlay)

(event Collision|EventActorBeginOverlap
  (params (OtherActor :type Actor%20Object%20Reference)))

(event EventTick
  (params (DeltaSeconds :type Float%20%28single-precision%29)))

(fn ConstructionScript)