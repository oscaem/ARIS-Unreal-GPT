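; BP_Table is the ship's lab table where the player synthesizes collected minerals.
; UpdateState shows the first three minerals from the game instance on slot meshes, updates BP_MineralCount, and enables CanSynth at three or more.
; When CanSynth is set, a box overlap registers the table as the player's interactable with a HUD prompt.
; Interaction runs Synthesize, stores success in SynthGood, then calls MineralsSynthesized.
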(event OnComponentBeginOverlap(Box)
  (params (OverlappedComponent :type Primitive%20Component%20Object%20Reference) (OtherActor :type Actor%20Object%20Reference) (OtherComp :type Primitive%20Component%20Object%20Reference) (OtherBodyIndex :type Integer) (bFromSweep :type Boolean) (SweepResult :type Hit%20Result%20Structure%20%28by%20ref%29))
  ;[1 1 1] EnableSynth
  (if (Variables|/Game/Core/GameInstanceFP.GameInstanceFP_C|GetCanSynth (CallFunction|GetDirectGameInstance))
    (bind _asbp_first_person_character (Utilities|Casting|CastToBP_FirstPersonCharacter OtherActor))
    (Variables|/Game/Actors/Player/BP_FirstPersonCharacter.BP_FirstPersonCharacter_C|SetCurrentInteractable _asbp_first_person_character self)
    (Default|DisplayActionPrompt (CallFunction|GetDirectHUDInterface) "SYNTHETISIEREN" true)
    (else
      (Development|PrintString "Not Enough Minerals To Synth"))))

(event OnComponentEndOverlap(Box)
  (params (OverlappedComponent :type Primitive%20Component%20Object%20Reference) (OtherActor :type Actor%20Object%20Reference) (OtherComp :type Primitive%20Component%20Object%20Reference) (OtherBodyIndex :type Integer))
  ;[1 1 1] EnableSynth
  (if (Variables|/Game/Core/GameInstanceFP.GameInstanceFP_C|GetCanSynth (CallFunction|GetDirectGameInstance))
    (bind _asbp_first_person_character (Utilities|Casting|CastToBP_FirstPersonCharacter OtherActor))
    (Variables|/Game/Actors/Player/BP_FirstPersonCharacter.BP_FirstPersonCharacter_C|SetCurrentInteractable _asbp_first_person_character 0)
    (Default|DisplayActionPrompt (CallFunction|GetDirectHUDInterface) "" false)))

(event EventUpdateState
  (bind _asgame_instance_fp (CallFunction|GetDirectGameInstance))
  (bind _collectedminerals (Variables|/Game/Core/GameInstanceFP.GameInstanceFP_C|GetCollectedMinerals _asgame_instance_fp))
  (bind _returnvalue (Utilities|Array|Length _collectedminerals))
  ;[1 1 1] UPDATE STATE
  (for (_array_element _array_index) _collectedminerals
    (CallFunction|UpdateDisplaySlot (Utilities|Enum|ByteToEnumMineral _array_element) _array_index)
    (bind _outactors (Actor|GetAllActorsOfClass "/Game/UserInterface/Other/WorldInterfaces/BP_MineralCount.BP_MineralCount_C"))
    (Default|SetCount (Utilities|Array|Get(acopy) _outactors) _returnvalue)
    (if (>= _returnvalue 3)
      (Variables|/Game/Core/GameInstanceFP.GameInstanceFP_C|SetCanSynth _asgame_instance_fp true)))
  (Development|PrintString "Updated Lab Display"))

(event EventInteraction
  (bind _asgame_instance_fp (CallFunction|GetDirectGameInstance))
  ;[1 1 1] Interact
  (bind _isgood (Default|Synthesize _asgame_instance_fp))
  (if _isgood
    (Variables|/Game/Core/GameInstanceFP.GameInstanceFP_C|SetSynthGood _asgame_instance_fp true)
    (Development|PrintString (Utilities|String|ToString(Boolean) _isgood))
    (else
      (Variables|/Game/Core/GameInstanceFP.GameInstanceFP_C|SetSynthGood _asgame_instance_fp false)
      (Development|PrintString (Utilities|String|ToString(Boolean) _isgood))))
  (Default|MineralsSynthesized (CallFunction|GetDirectGameInstance)))

(fn ConstructionScript)

(fn UpdateDisplaySlot
  (params (Mineral :type Mineral%20Enum :default "NewEnumerator0") (Index :type Integer))
  (if (<= Index 2)
    (switch Utilities|FlowControl|Switch|SwitchonMineral Mineral
      (:NewEnumerator0
        (CallFunction|GetMineralIndex Index "/Game/Actors/Minerals/Meshes/DemoSample.DemoSample" "/Game/Actors/Minerals/Materials/Instances/MI_Mineral_Tropium.MI_Mineral_Tropium"))
      (:NewEnumerator1
        (CallFunction|GetMineralIndex Index "/Game/Actors/Minerals/Meshes/DemoSample.DemoSample" "/Game/Actors/Minerals/Materials/Instances/MI_Mineral_Trinit.MI_Mineral_Trinit"))
      (:NewEnumerator2
        (CallFunction|GetMineralIndex Index "/Game/Actors/Minerals/Meshes/DemoSample.DemoSample" "/Game/Actors/Minerals/Materials/Instances/MI_Mineral_Fusium.MI_Mineral_Fusium"))
      (:NewEnumerator3
        (CallFunction|GetMineralIndex Index "/Game/Actors/Minerals/Meshes/DemoSample.DemoSample" "/Game/Actors/Minerals/Materials/Instances/MI_Mineral_Palladium.MI_Mineral_Palladium"))
      (:NewEnumerator4
        (CallFunction|GetMineralIndex Index "/Game/Actors/Minerals/Meshes/DemoSample.DemoSample" "/Game/Actors/Minerals/Materials/Instances/MI_Mineral_Fusionit.MI_Mineral_Fusionit"))
      (:NewEnumerator5
        (CallFunction|GetMineralIndex 0 "/Game/Actors/Minerals/Meshes/DemoSample.DemoSample" "/Game/Actors/Minerals/Materials/Instances/MI_Mineral_Peperium.MI_Mineral_Peperium")))))

(fn GetMineralIndex
  (params (Index :type Integer) (Mesh :type Static%20Mesh%20Object%20Reference) (Material :type Material%20Instance%20Object%20Reference))
  (bind _slot1 (Variables|Default|GetSlot1))
  (bind _slot2 (Variables|Default|GetSlot2))
  (bind _slot3 (Variables|Default|GetSlot3))
  (switch int Index
    (:0
      (Components|StaticMesh|SetStaticMesh _slot1 Mesh)
      (Rendering|Material|SetMaterial _slot1 0 Material))
    (:1
      (Components|StaticMesh|SetStaticMesh _slot2 Mesh)
      (Rendering|Material|SetMaterial _slot2 0 Material))
    (:2
      (Components|StaticMesh|SetStaticMesh _slot3 Mesh)
      (Rendering|Material|SetMaterial _slot3 0 Material))))