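; Side quest Blueprint X03, completed in the quest log once the player has collected at least one artifact and at least one mineral.
; BeginPlay binds to the Game Instance's artifact and mineral collection events; the parent BeginPlay call is left unconnected.
; Each handler checks both collection arrays through count-threshold macros, then either completes the quest or prints which item is still missing.
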(event Custom|OnArtifactCollected
  (|MoreArtifactsThan
    (:true
      (|MoreMineralsThan_2
        (:true
          (Default|CompleteQuest (CallFunction|GetDirectQuestLogComponent) (Variables|Default|GetQuestID)))
        (:false
          (Development|PrintString "Collect a Mineral!"))))))

(event Custom|OnMineralCollected
  (|MoreMineralsThan
    (:true
      (|MoreArtifactsThan_2
        (:true
          (Default|CompleteQuest (CallFunction|GetDirectQuestLogComponent) (Variables|Default|GetQuestID)))
        (:false
          (Development|PrintString "Collect an Artifact"))))))

(event EventBeginPlay
  (bind _asgame_instance_fp (CallFunction|GetDirectGameInstance))
  (EventDispatchers|BindEventtoOnArtifactCollected _asgame_instance_fp (delegate Custom|OnArtifactCollected))
  (EventDispatchers|BindEventtoOnMineralCollected _asgame_instance_fp (delegate Custom|OnMineralCollected)))

(fn ConstructionScript
  (|CallParentFunction))