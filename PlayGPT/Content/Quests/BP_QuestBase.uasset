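; BP_QuestBase is a quest Blueprint that loads its own details from a data table when play begins.
; BeginPlay calls PullQuestDetailsFromTable, which looks up the row referenced by the QuestData row handle.
; When the row is found, it copies the name, ID, tracking description, main-quest flag and act ID into its variables.
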(event EventBeginPlay
  (CallFunction|PullQuestDetailsfromTable))

(fn ConstructionScript)

(fn PullQuestDetailsfromTable
  (bind _questdata (Variables|Details|GetQuestData))
  (bind (_datatable _rowname) (Utilities|Struct|BreakDataTableRowHandle _questdata))
  (bind _returnvalue (Utilities|GetDataTableRow _datatable _rowname)
    (:then
      (Variables|Details|SetQuestName (.Name (Utilities|Struct|BreakFQuest _returnvalue)))
      (Variables|Details|SetQuestID (.QuestID (Utilities|Struct|BreakFQuest _returnvalue)))
      (Variables|Details|SetQuestDescription (.TrackingDescription (Utilities|Struct|BreakFQuest _returnvalue)))
      (Variables|Details|SetisMainQuest (.isMainQuest (Utilities|Struct|BreakFQuest _returnvalue)))
      (Variables|Details|SetActID (.ActID (Utilities|Struct|BreakFQuest _returnvalue))))))