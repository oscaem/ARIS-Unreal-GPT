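; BP_Quest_107 is the final quest, which selects and plays the game's ending through GameInstance events.
; On arrival at a specific level, it picks an ending from Sola retrieval, collected minerals and artifact count, then plays the death or return cutscene.
; The return hands back control for fuel synthesis, whose result triggers the good or bad cinematic.
; When an ending cinematic finishes, it shows credits and completes the quest.
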(event Custom|Completed
  (params (ToLevel :type Level%20Enum :default "NewEnumerator0"))
  (bind _asgame_instance_fp (CallFunction|GetDirectGameInstance))
  (bind _collectedartifacts (Variables|/Game/Core/GameInstanceFP.GameInstanceFP_C|GetCollectedArtifacts _asgame_instance_fp))
  (bind _returnvalue (Utilities|Array|Length _collectedartifacts))
  ;[1 1 1 1 40] PLAY SYNTH CUTSCENE
  (if (Utilities|Enum|Equal(Enum) ToLevel "NewEnumerator0")
    (if (Variables|/Game/Core/GameInstanceFP.GameInstanceFP_C|GetSolaRetreived _asgame_instance_fp)
      (Development|PrintString "SOLA ENDING")
      (Variables|/Game/Core/GameInstanceFP.GameInstanceFP_C|SetCurrentEnding (CallFunction|GetDirectGameInstance) "NewEnumerator1")
      (Variables|Default|SetEndingDialogue "TrinitWildcard")
      (elif (Utilities|Array|ContainsItem (Variables|/Game/Core/GameInstanceFP.GameInstanceFP_C|GetCollectedMinerals _asgame_instance_fp) "NewEnumerator1")
        (Development|PrintString "TRINIT WILDCARD ENDING")
        (Variables|/Game/Core/GameInstanceFP.GameInstanceFP_C|SetCurrentEnding (CallFunction|GetDirectGameInstance) "NewEnumerator2")
        (Variables|Default|SetEndingDialogue "TrinitWildcard")
        (elif (< _returnvalue 3)
          (Development|PrintString "DEATH ENDING")
          (Variables|/Game/Core/GameInstanceFP.GameInstanceFP_C|SetCurrentEnding (CallFunction|GetDirectGameInstance) "NewEnumerator3")
          (Variables|Default|SetEndingDialogue "DeadEnd")
          (elif (< _returnvalue 9)
            (Development|PrintString "REGULAR ENDING")
            (Variables|/Game/Core/GameInstanceFP.GameInstanceFP_C|SetCurrentEnding (CallFunction|GetDirectGameInstance) "NewEnumerator4")
            (Variables|Default|SetEndingDialogue "AfterLastReturn")
            (else
              (Development|PrintString "10 ARTIFACT ENDING")
              (Variables|/Game/Core/GameInstanceFP.GameInstanceFP_C|SetCurrentEnding (CallFunction|GetDirectGameInstance) "NewEnumerator5")
              (Variables|Default|SetEndingDialogue "10ArtEnding"))))))
    (Default|AnimationLock (.ARIS (CallFunction|GetDirectARIS)) true)
    (if (Utilities|Enum|Equal(Enum) (Variables|/Game/Core/GameInstanceFP.GameInstanceFP_C|GetCurrentEnding (CallFunction|GetDirectGameInstance)) "NewEnumerator3")
      (Default|PlaySequence (CallFunction|GetDirectGameInstance) "/Game/Movies/Endings/Cin_Ending_DeathEnding.Cin_Ending_DeathEnding")
      (Game|SpawnActorfromClass "/Game/Movies/SpecialEffects/CinematicActors/BP_FailureLight.BP_FailureLight_C" (Math|Transform|MakeTransform "1000.000000,200.000000,600.000000") "Undefined" "MultiplyWithRoot" 0 0)
      (else
        (CallFunction|PlayScriptedARIS (Variables|Default|GetEndingDialogue))
        (Default|PlaySequence (CallFunction|GetDirectGameInstance) "/Game/Movies/Cin_FinalReturn.Cin_FinalReturn")))))

(event Custom|OnMaterialSynthesized
  ;[0 0 0 1 40] PLAY FINAL CUTSCENE
  (Variables|/Game/Actors/NPCs/BP_NPC_ARIS.BP_NPC_ARIS_C|SetlocksOn (.ARIS (CallFunction|GetDirectARIS)) false)
  (Widget|RemovefromParent (CallFunction|GetDirectHUDInterface))
  (if (Variables|/Game/Core/GameInstanceFP.GameInstanceFP_C|GetSynthGood (CallFunction|GetDirectGameInstance))
    (CallFunction|PlayScriptedARIS "None")
    (Default|PlaySequence (CallFunction|GetDirectGameInstance) "/Game/Movies/Endings/Cin_Ending_Good_RegularTrinitSola10.Cin_Ending_Good_RegularTrinitSola10")
    (bind _outactors (Actor|GetAllActorsOfClass "/Script/Engine.AmbientSound"))
    (for _array_element _outactors
      (Actor|DestroyActor _array_element))
    (else
      (CallFunction|PlayScriptedARIS "None")
      (Default|PlaySequence (CallFunction|GetDirectGameInstance) "/Game/Movies/Endings/Cin_Ending_RegularBad.Cin_Ending_RegularBad")
      (Game|SpawnActorfromClass "/Game/Movies/SpecialEffects/CinematicActors/BP_ErrorLight.BP_ErrorLight_C" (Math|Transform|MakeTransform "-1600.000000,-110.000000,20.000000") "Undefined" "MultiplyWithRoot" 0 0))))

(event Custom|OnCutsceneEnded
  (params (PlayedCutscene :type Level%20Sequence%20Actor%20Object%20Reference))
  (bind _returnvalue (Class|LevelSequenceActor|GetSequence PlayedCutscene))
  (if (== _returnvalue "/Game/Movies/Cin_FinalReturn.Cin_FinalReturn")
    (CallFunction|RepossessPlayer)
    (Default|AnimationLock (.ARIS (CallFunction|GetDirectARIS)) false)
    (Variables|/Script/UMG.TextBlock|SetText (Variables|/Game/UserInterface/HUD/UIPlayerHUD.UIPlayerHUD_C|GetMainQuestInfo (CallFunction|GetDirectHUDInterface)) "Synthetisiere den Treibstoff")
    (elif (== _returnvalue "/Game/Movies/Endings/Cin_Ending_DeathEnding.Cin_Ending_DeathEnding")
      (CallFunction|TriggerGameEnd :!label _label)
      (Default|CompleteQuest (CallFunction|GetDirectQuestLogComponent) (.RowName (Utilities|Struct|BreakDataTableRowHandle (Variables|Default|GetQuestData))))
      (elif (== _returnvalue "/Game/Movies/Endings/Cin_Ending_RegularBad.Cin_Ending_RegularBad")
        (Development|PrintString "Bad Ending")
        (goto _label)
        (elif (== _returnvalue "/Game/Movies/Endings/Cin_Ending_Good_RegularTrinitSola10.Cin_Ending_Good_RegularTrinitSola10")
          (goto _label)
          (else
            (Development|PrintString "Wrong Sequence Loaded")))))))

(event EventBeginPlay
  (bind _asgame_instance_fp (CallFunction|GetDirectGameInstance))
  ;[1 1 1 1 40] CREATE CALLBACKS
  (EventDispatchers|BindEventtoOnLevelChanged _asgame_instance_fp (delegate Custom|Completed))
  (EventDispatchers|BindEventtoOnMineralsSynthesized _asgame_instance_fp (delegate Custom|OnMaterialSynthesized))
  (EventDispatchers|BindEventtoOnCutsceneEnded _asgame_instance_fp (delegate Custom|OnCutsceneEnded)))

(fn ConstructionScript
  (|CallParentFunction))

(fn TriggerReturnCutscene
  (params (RowName :type Name))
  (Default|AnimationLock (.ARIS (CallFunction|GetDirectARIS)) true)
  (if (Utilities|Enum|Equal(Enum) (Variables|/Game/Core/GameInstanceFP.GameInstanceFP_C|GetCurrentEnding (CallFunction|GetDirectGameInstance)) "NewEnumerator3")
    (CallFunction|PlayScriptedARIS "DeadEnd")
    (bind _outactor (Sequencer|Player|CreateLevelSequencePlayer "/Game/Movies/Endings/Cin_Ending_DeathEnding.Cin_Ending_DeathEnding"))
    (bind _output_get (LocalVariables|SetCineActor _outactor))
    (Sequencer|Player|Play (Variables|/Script/LevelSequence.LevelSequenceActor|GetSequencePlayer _output_get) :!class /Script/MovieScene.MovieSceneSequencePlayer)
    (CallFunction|TriggerGameEnd)
    (Default|CompleteQuest (CallFunction|GetDirectQuestLogComponent) (.RowName (Utilities|Struct|BreakDataTableRowHandle (Variables|Default|GetQuestData))))
    (else
      (CallFunction|PlayScriptedARIS RowName)
      (bind _outactor_2 (Sequencer|Player|CreateLevelSequencePlayer "/Game/Movies/Cin_FinalReturn.Cin_FinalReturn"))
      (bind _output_get_2 (LocalVariables|SetCineActor _outactor_2))
      (Sequencer|Player|Play (Variables|/Script/LevelSequence.LevelSequenceActor|GetSequencePlayer _output_get_2) :!class /Script/MovieScene.MovieSceneSequencePlayer)
      (return (Class|TimeManagementBlueprintLibrary|ToSeconds(QualifiedFrameTime) (Media|MediaPlayer|GetDuration (Variables|/Script/LevelSequence.LevelSequenceActor|GetSequencePlayer _output_get_2)))))))

(fn TriggerGameEnd
  (bind _returnvalue (UserInterface|CreateWidget "/Game/UserInterface/EndCredits/EndCredits.EndCredits_C" (Game|GetPlayerController 0)))
  (UserInterface|Viewport|AddtoViewport _returnvalue 100000))