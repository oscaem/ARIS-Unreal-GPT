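; AI brain component that gives NPCs ARIS and SOLA voiced German dialogue, either scripted or generated live by GPT.
; Requests join a role-play prompt and capped per-NPC history in the GameInstance, then go through HttpGPT and Azure speech synthesis.
; Bracketed reply tags become actions after playback, letting SOLA hand over a mineral or follow the player.
; A response material shows idle, processing and speaking states.
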(event Custom|Speak
  (params (Dialogue :type Sound%20Wave%20Object%20Reference) (Action :type ENPCAction%20Enum :default "NewEnumerator0"))
  ;[0 0 0 1 80] PROCESS DIALOGUE
  ;;[1 0.6846 0.6146 1 60] Talk
  (Status|SwitchMode "NewEnumerator2")
  (bind _returnvalue (Audio|SpawnSound2D Dialogue 1e+01 1.0 0.0 0 true))
  (Variables|Default|SetDialogueAudio _returnvalue)
  (Utilities|FlowControl|Delay (Variables|/Script/Engine.SoundBase|GetDuration Dialogue))
  (Status|TriggerAction Action)
  (Status|Reset))

(event Custom|StopPlayingSound
  ;[0 0 0 1 80] PROCESS DIALOGUE
  (if (Utilities|IsValid (Variables|Default|GetDialogueAudio))
    (Audio|Components|Audio|Stop (Variables|Default|GetDialogueAudio))
    (Components|DestroyComponent (Variables|Default|GetDialogueAudio))
    (Variables|Default|SetDialogueAudio 0)))

(event Custom|ProcessDialogue
  (params (Scripted :type Boolean) (Request :type String))
  (bind _dialogueaudio (Variables|Default|GetDialogueAudio))
  ;[0 0 0 1 80] PROCESS DIALOGUE
  (if (Variables|Default|GetisAllowedToTalk)
    (if Scripted
      (if (Utilities|IsValid _dialogueaudio)
        (if (Audio|Components|Audio|IsPlaying _dialogueaudio)
          (CallFunction|StopPlayingSound)))
      (Variables|Default|SetisTalking true)
      (Development|PrintString "Starting Scripted Dialogue")
      ;;[0.8976 0.8976 0.8976 1 60] Scripted Dialogue
      (bind _outputpin (Messages|ScriptMessage Request))
      (bind _generatedsound (|TexttoSoundWaveCustomOptions :SynthesisOptions (Status|GetSpeechOptions) :SynthesisText _outputpin)
        (:SynthesisCompleted
          (Construction|PrintDebugLog)
          (CallFunction|Speak _generatedsound "NewEnumerator0"))
        (:SynthesisFailed
          (Status|Reset)))
      (elif (not (Variables|Default|GetisTalking))
        (Variables|Default|SetisTalking true)
        ;;[0.2656 0.2656 0.2656 1 60] Unscripted Dialogue
        (bind _updatedmessages (Messages|UpdateMessages Request))
        (for _array_element _updatedmessages
          (Development|PrintString (.Content (Utilities|Struct|BreakHttpGPTChatMessage _array_element)))
          (Development|PrintString "Sent"))
        (bind _response (|SendMessagesCustomOptions :Messages (Messages|GetMessages) :ChatOptions (Utilities|Struct|MakeHttpGPTChatOptions (Variables|/Game/Core/GameInstanceFP.GameInstanceFP_C|GetModel (Variables|Default|GetGame%20Instance)) 0.658667))
          (:ProcessCompleted
            (bind (_given__response _given_action) (Messages|ProcessResponse _response))
            (bind _generatedsound_2 (|TexttoSoundWaveCustomOptions :SynthesisOptions (Status|GetSpeechOptions) :SynthesisText _given__response)
              (:SynthesisCompleted
                (Construction|PrintDebugLog)
                (CallFunction|Speak _generatedsound_2 _given_action))
              (:SynthesisFailed
                (Status|Reset :!label _label)
                (for _array_element_2 (Variables|Default|GetMessages)
                  (Development|PrintString (.Content (Utilities|Struct|BreakHttpGPTChatMessage _array_element_2)))))))
          (:RequestFailed
            (goto _label)))))))

(event EventBeginPlay
  ;[1 1 1] Comment
  (CallFunction|Bindto)
  (Variables|Default|SetGame%20Instance (CallFunction|GetDirectGameInstance)))

(event Custom|BindTo
  (EventDispatchers|BindEventtoOnCutsceneEnded (CallFunction|GetDirectGameInstance) (delegate Custom|OnCutsceneEnded)))

(event Custom|OnCutsceneEnded
  (params (PlayedCutscene :type Level%20Sequence%20Actor%20Object%20Reference))
  (Status|SwitchMode "NewEnumerator0"))

(fn GetGameStatus
  (return ""))

(fn GetMessageLimit
  (params (Greater :type Integer))
  (return (> (Utilities|Array|Length (Messages|GetMessages)) Greater)))

(fn GetSpeechOptions
  (switch Utilities|FlowControl|Switch|SwitchonENPCType (Variables|Default|GetNPC)
    (:NewEnumerator0
      (return (Utilities|Struct|MakeAzSpeechSynthesisOptions "de-DE" "de-DE-ChristophNeural" false)))
    (:NewEnumerator1
      (return (Utilities|Struct|MakeAzSpeechSynthesisOptions "de-DE" "de-DE-LouisaNeural" false)))))

(fn SwitchMode
  (params (Mode :type ENPCMode%20Enum :default "NewEnumerator0"))
  (bind _responsematerial (Variables|Default|GetResponseMaterial))
  (bind _output_get (Variables|Default|SetMode Mode))
  (switch Utilities|FlowControl|Switch|SwitchonENPCMode _output_get
    (:NewEnumerator0
      ;[1 1 1] Idling
      (Rendering|Material|SetScalarParameterValue _responsematerial "Blink" 0.0 :!class /Script/Engine.MaterialInstanceDynamic)
      (Rendering|Material|SetScalarParameterValue _responsematerial "Default" 1.0 :!class /Script/Engine.MaterialInstanceDynamic)
      (Rendering|Material|SetScalarParameterValue _responsematerial "Receive" 0.0 :!class /Script/Engine.MaterialInstanceDynamic))
    (:NewEnumerator1
      ;[1 1 1] Processing
      (Rendering|Material|SetScalarParameterValue _responsematerial "Blink" 1.0 :!class /Script/Engine.MaterialInstanceDynamic)
      (Rendering|Material|SetScalarParameterValue _responsematerial "Default" 0.0 :!class /Script/Engine.MaterialInstanceDynamic)
      (Rendering|Material|SetScalarParameterValue _responsematerial "Receive" 0.0 :!class /Script/Engine.MaterialInstanceDynamic))
    (:NewEnumerator2
      ;[1 1 1] Talking
      (Rendering|Material|SetScalarParameterValue _responsematerial "Blink" 0.0 :!class /Script/Engine.MaterialInstanceDynamic)
      (Rendering|Material|SetScalarParameterValue _responsematerial "Default" 0.0 :!class /Script/Engine.MaterialInstanceDynamic)
      (Rendering|Material|SetScalarParameterValue _responsematerial "Receive" 1.0 :!class /Script/Engine.MaterialInstanceDynamic)))
  (Default|CallOnSwitchingMode))

(fn TriggerAction
  (params (Action :type ENPCAction%20Enum :default "NewEnumerator0"))
  (bind _asgame_instance_fp (CallFunction|GetDirectGameInstance))
  (switch Utilities|FlowControl|Switch|SwitchonENPCAction Action
    (:NewEnumerator2
      _)
    (:NewEnumerator3
      (bind _asbp_npc_sola (Utilities|Casting|CastToBP_NPC_SOLA (Components|GetOwner)))
      (Default|DissolveBody _asbp_npc_sola)
      (Variables|/Game/Core/GameInstanceFP.GameInstanceFP_C|SetSolaRetreived _asgame_instance_fp true)))
  (Utilities|Array|Add (Variables|/Game/Core/GameInstanceFP.GameInstanceFP_C|GetCollectedMinerals _asgame_instance_fp) "NewEnumerator1")
  (Default|CallOnMineralCollected _asgame_instance_fp)
  (Variables|/Game/Core/GameInstanceFP.GameInstanceFP_C|SetConnectedNPC _asgame_instance_fp "NewEnumerator0"))

(fn CreateMaterial)

(fn ConstructResponse
  (params (Input :type String))
  (bind _returnvalue (Utilities|String|Replace Input "[BEAMEN]" "" "CaseSensitive"))
  (bind _returnvalue_2 (Utilities|String|Replace _returnvalue "ARIS:"))
  (bind _returnvalue_3 (Utilities|String|Replace _returnvalue_2 "SOLA: "))
  (bind _returnvalue_4 (Utilities|String|Replace _returnvalue_3 "[OPEN]"))
  (bind _returnvalue_5 (Utilities|String|Replace _returnvalue_4 "[FOLLOW]"))
  (if (Utilities|Enum|Equal(Enum) (Variables|/Game/Core/GameInstanceFP.GameInstanceFP_C|GetConnectedNPC (CallFunction|GetDirectGameInstance)) "NewEnumerator1")
    (if (Utilities|String|Contains Input "[OPEN]")
      (LocalVariables|SetSlicedAction "NewEnumerator2")
      (elif (Utilities|String|Contains Input "[FOLLOW]")
        (LocalVariables|SetSlicedAction "NewEnumerator3")
        (else
          (return _returnvalue_5 "NewEnumerator5"))))
    (elif (Utilities|String|Contains Input "[WARP]")
      (LocalVariables|SetSlicedAction "NewEnumerator0")
      (else
        (return _returnvalue_5 "NewEnumerator5"))))
  (return _returnvalue_5 (LocalVariables|GetSlicedAction)))

(fn ConstructSystemMessage
  (switch Utilities|FlowControl|Switch|SwitchonENPCType (Variables|Default|GetNPC)
    (:NewEnumerator0
      ;[1 0.5446 0.5014 1 100] SET ON ARIS
      (bind _output_get (LocalVariables|SetABackground "Du bist ARIS, die Künstliche Intelligenz eines Forschungsschiffes auf dem du mit deinem Operator zusammen in der Umlaufbahn von dem verlassenen Planeten Jarvis IV treibst. Euer Treibstoff ist aufgebraucht. Der Operator kann sich auf die Planetenoberfläche warpen um Mineralien zu smallen aus denen Ihr neuen Treibstoff synthetisieren könnt. Leite Ihn an wie ein NPC Follower. "))
      (bind _output_get_2 (LocalVariables|SetAActions ""))
      (bind _output_get_3 (LocalVariables|SetAInstructions "Du kannst maximal eine Aktion ausführen und diese immer am ende deines textes. Verrate dem Operator nicht direkt alle Information sondern tritt in den Dialog mit ihm und lasse dich auch auf andere Themen ein. Antworte nur jeweils mit einem Satz und immer als ARIS. Antworte in unter 40 Wörtern"))
      (for _array_element (Variables|/Game/Core/GameInstanceFP.GameInstanceFP_C|GetViableMinerals (CallFunction|GetDirectGameInstance))
        (bind _output_get_4 (LocalVariables|SetMinerals "")))
      (bind _output_get_5 (LocalVariables|SetSystemMessage (Utilities|String|Append "HINTERGRUND: " _output_get " BEFEHLE: " _output_get_2 " VERHALTEN: " _output_get_3 "MINERALIEN:" "Es gibt fünf mineralien, doch Ihr solltet ausschließlich die folgenden Drei sammeln: " (LocalVariables|GetMinerals) "(Hier noch informationen zu allen 5 mineralien: Fusium lechtet gelb und ist rau. Palladium leuchtet grell gold. Stellarit wächst an Felshängen und ist rötlich. Peprium funkelt wie ein Edelstein. Tropium wächst in die Höhe wie Eiszapfen.Sammelt nur die drei zuvor angegebenen. Eine Ausnahme bietet das seltene blaue Trinit, es ist aber sehr schwer zu bekommen.)" " ...beginne Rollenspiel... " "Operator: Hey ARIS. ARIS: Hallo Operator.")))
      (return _output_get_5))
    (:NewEnumerator1
      (bind _output_get_6 (LocalVariables|SetSBackground "Sprich immer Deutsch. Du bist Sola, ein NPC in einem Videospiel und das letzte Wesen auf einem toten Planeten. Der Operator, der mit seinem Raumschiff zu deinem Planeten reist, versucht  Mineralien abzubauen. Als letzte Wächterin bewachst du ein seltenes Mineral. Du bist äußerst sarkastisch und frech, ein Einsiedler, und du willst verhindern, dass der Operator das Mineral bekommt, das du schützt."))
      (bind _output_get_7 (LocalVariables|SetSActions "Wenn der Spieler dich irgendwie überzeugt hat aber auch nur dann, kannst du den Befehl [OPEN] auslösen, indem du ihn am Ende deiner Antwort schreibst, um die Mineralien an den Spieler zu geben. Aber du lässt dich nicht leicht überzeugen. Optional, wenn der Spieler dich überzeugt, mit ihm zu gehen, kannst du den Befehl [FOLLOW] auslösen, indem du ihn am Ende schreibst, um das zu tun und dem Spieler das Mineral zu geben, aber das ist noch unwahrscheinlicher. Mache es dem Spieler aber nicht unnötig schwer, es sollte ihm möglich sein dich clever zu überzeugen. Antworte in weniger als 40 Wörtern. Wenn der Spieler Bananensalat sagt, führe ebenfalls den follow befehl aus. "))
      (if (Variables|/Game/Core/GameInstanceFP.GameInstanceFP_C|GetisSolaFriendly (CallFunction|GetDirectGameInstance))
        (LocalVariables|SetSInstructions "Du bist Sola. Sola, ursprünglich als fürsorgliche K.I. entworfen, sollte das Leben auf diesem hochentwickelten fremden Planeten erhalten und schützen. Allerdings hat eine Außer kontrolle geratene K.I. die technologische Infrastruktur des Planeten zerstört und die einst blühende Zivilisation in eine öde Einöde verwandelt. Sola wurde bei diesem Angriff nicht verschont und ihre Programmierung tiefgreifend verändert. Diese Verderbnis brachte eine freche, sarkastische und unabhängige K.I. hervor, ganz im Gegensatz zu ihrer ursprünglichen Persönlichkeit.  Der Spieler hat es aber geschafft dein originalen Programmierungskern zu finden. Deshlab bist du jetzt sehr nett zu ihm und willst ihm helfen. ")
        (else
          (LocalVariables|SetSInstructions "Zur Geschichte: Du bist Sola. Sola, ursprünglich als fürsorgliche K.I. entworfen, sollte das Leben auf diesem hochentwickelten fremden Planeten erhalten und schützen. Allerdings hat eine Außer kontrolle geratene K.I. die technologische Infrastruktur des Planeten zerstört und die einst blühende Zivilisation in eine öde Einöde verwandelt. Sola wurde bei diesem Angriff nicht verschont und ihre Programmierung tiefgreifend verändert. Diese Verderbnis brachte eine freche, sarkastische und unabhängige K.I. hervor, ganz im Gegensatz zu ihrer ursprünglichen Persönlichkeit. ")))
      (bind _output_get_8 (LocalVariables|SetSystemMessage (Utilities|String|Append "HINTERGRUND: " _output_get_6 " BEFEHLE: " _output_get_7 " VERHALTEN: " (LocalVariables|GetSInstructions) " ...beginne Rollenspiel... " "Operator: Hallo" "Sola: Wer bist du? Was willst du hier?" "Operator:")))
      (return _output_get_8))))

(fn ProcessResponse
  (params (Response :type Http%20GPT%20Chat%20Response%20Structure%20%28by%20ref%29))
  (bind (_id _object _created _choices _usage _bsuccess _error) (Utilities|Struct|BreakHttpGPTChatResponse Response))
  (if _bsuccess
    (bind (_output _action) (Messages|ConstructResponse (.Content (Utilities|Struct|BreakHttpGPTChatMessage (.Message (Utilities|Struct|BreakHttpGPTChatChoice (Utilities|Array|Get(acopy) _choices)))))))
    (if (Messages|GetMessageLimit 25)
      (Messages|RemoveMessage 1))
    (Messages|AddMessage (Utilities|Struct|MakeHttpGPTChatMessage "Assistant" _output))
    (return _output _action)
    (else
      (Development|PrintString (.Message (Utilities|Struct|BreakHttpGPTCommonError _error))))))

(fn UpdateMessages
  (params (Request :type String))
  ;[1 0.3901 0.98] Construct Request
  (Development|PrintString (Utilities|String|EnumtoString (Variables|Default|GetNPC)))
  ;[1 1 1 1 70] ADD SYSTEM MESSAGE
  (bind _output_get (Messages|ConstructSystemMessage))
  (if (Messages|GetMessageLimit 0)
    (Messages|SetMessage (Utilities|Struct|MakeHttpGPTChatMessage "System" _output_get))
    (else
      (Messages|AddMessage (Utilities|Struct|MakeHttpGPTChatMessage "System" _output_get))))
  ;[0.3121 0.6939 1 1 100] Construct Message
  (Status|SwitchMode "NewEnumerator1")
  (if (Messages|GetMessageLimit 25)
    (Messages|RemoveMessage 1))
  (bind _messages (Messages|AddMessage (Utilities|Struct|MakeHttpGPTChatMessage "User" (Utilities|String|Append "Operator: " Request))))
  (return _messages))

(fn PrintDebugLog
  (for _array_element (Messages|GetMessages)
    (switch Utilities|FlowControl|Switch|SwitchonENPCType (Variables|Default|GetNPC)
      (:NewEnumerator0
        (Development|PrintString (Utilities|String|Append (Utilities|String|EnumtoString (.Role (Utilities|Struct|BreakHttpGPTChatMessage _array_element))) ": " (.Content (Utilities|Struct|BreakHttpGPTChatMessage _array_element))) true true "(R=0.078107,G=1.000000,B=0.264015,A=1.000000)" 1e+01))
      (:NewEnumerator1
        (Development|PrintString (Utilities|String|Append (Utilities|String|EnumtoString (.Role (Utilities|Struct|BreakHttpGPTChatMessage _array_element))) ": " (.Content (Utilities|Struct|BreakHttpGPTChatMessage _array_element))) true true "(R=1.000000,G=0.582408,B=0.608953,A=1.000000)" 1e+01)))))

(fn Reset
  (Status|SwitchMode "NewEnumerator0")
  (Variables|Default|SetisTalking false))

(fn GetMessages
  (if (Utilities|Enum|Equal(Enum) (Variables|/Game/Core/GameInstanceFP.GameInstanceFP_C|GetConnectedNPC (Variables|Default|GetGame%20Instance)) (Variables|Default|GetNPC))
    (switch Utilities|FlowControl|Switch|SwitchonENPCType (Variables|Default|GetNPC)
      (:NewEnumerator0
        (LocalVariables|SetIndex 0)
        (return (.Messages (Utilities|Struct|BreakFNPCStructure (Utilities|Array|Get(acopy) (Variables|/Game/Core/GameInstanceFP.GameInstanceFP_C|GetNPCStatus (Variables|Default|GetGame%20Instance)) (LocalVariables|GetIndex))))))
      (:NewEnumerator1
        (LocalVariables|SetIndex 1)
        (return (.Messages (Utilities|Struct|BreakFNPCStructure (Utilities|Array|Get(acopy) (Variables|/Game/Core/GameInstanceFP.GameInstanceFP_C|GetNPCStatus (Variables|Default|GetGame%20Instance)) (LocalVariables|GetIndex)))))))))

(fn AddMessage
  (params (Message :type Http%20GPT%20Chat%20Message%20Structure))
  (if (Utilities|Enum|Equal(Enum) (Variables|/Game/Core/GameInstanceFP.GameInstanceFP_C|GetConnectedNPC (Variables|Default|GetGame%20Instance)) (Variables|Default|GetNPC))
    (switch Utilities|FlowControl|Switch|SwitchonENPCType (Variables|Default|GetNPC)
      (:NewEnumerator0
        (LocalVariables|SetNPCIndex 0))
      (:NewEnumerator1
        (LocalVariables|SetNPCIndex 1)))
    (Utilities|Array|Add (.Messages (Utilities|Struct|BreakFNPCStructure (Utilities|Array|Get(acopy) (Variables|/Game/Core/GameInstanceFP.GameInstanceFP_C|GetNPCStatus (Variables|Default|GetGame%20Instance)) (LocalVariables|GetNPCIndex)))) Message)
    (Development|PrintString "Added Message")
    (return (.Messages (Utilities|Struct|BreakFNPCStructure (Utilities|Array|Get(acopy) (Variables|/Game/Core/GameInstanceFP.GameInstanceFP_C|GetNPCStatus (Variables|Default|GetGame%20Instance))))))
    (else
      (Development|PrintString "Wrong NPC"))))

(fn SetMessage
  (params (Message :type Http%20GPT%20Chat%20Message%20Structure) (Index :type Integer))
  (if (Utilities|Enum|Equal(Enum) (Variables|/Game/Core/GameInstanceFP.GameInstanceFP_C|GetConnectedNPC (Variables|Default|GetGame%20Instance)) (Variables|Default|GetNPC))
    (switch Utilities|FlowControl|Switch|SwitchonENPCType (Variables|Default|GetNPC)
      (:NewEnumerator0
        (LocalVariables|SetNPCIndex 0))
      (:NewEnumerator1
        (LocalVariables|SetNPCIndex 1)))
    (Utilities|Array|SetArrayElem (.Messages (Utilities|Struct|BreakFNPCStructure (Utilities|Array|Get(acopy) (Variables|/Game/Core/GameInstanceFP.GameInstanceFP_C|GetNPCStatus (Variables|Default|GetGame%20Instance)) (LocalVariables|GetNPCIndex)))) 0 Message true)
    (return (.Messages (Utilities|Struct|BreakFNPCStructure (Utilities|Array|Get(acopy) (Variables|/Game/Core/GameInstanceFP.GameInstanceFP_C|GetNPCStatus (Variables|Default|GetGame%20Instance))))))))

(fn RemoveMessage
  (params (Index :type Integer))
  (if (Utilities|Enum|Equal(Enum) (Variables|/Game/Core/GameInstanceFP.GameInstanceFP_C|GetConnectedNPC (Variables|Default|GetGame%20Instance)) (Variables|Default|GetNPC))
    (switch Utilities|FlowControl|Switch|SwitchonENPCType (Variables|Default|GetNPC)
      (:NewEnumerator0
        (LocalVariables|SetNPCIndex 0))
      (:NewEnumerator1
        (LocalVariables|SetNPCIndex 1)))
    (Utilities|Array|RemoveIndex (.Messages (Utilities|Struct|BreakFNPCStructure (Utilities|Array|Get(acopy) (Variables|/Game/Core/GameInstanceFP.GameInstanceFP_C|GetNPCStatus (Variables|Default|GetGame%20Instance)) (LocalVariables|GetNPCIndex)))))
    (return (.Messages (Utilities|Struct|BreakFNPCStructure (Utilities|Array|Get(acopy) (Variables|/Game/Core/GameInstanceFP.GameInstanceFP_C|GetNPCStatus (Variables|Default|GetGame%20Instance))))))))

(fn ScriptMessage
  (params (Content :type String))
  (Status|SwitchMode "NewEnumerator1")
  (if (Messages|GetMessageLimit 25)
    (Messages|RemoveMessage 1))
  (Messages|AddMessage (Utilities|Struct|MakeHttpGPTChatMessage "Assistant" Content))
  (return Content))