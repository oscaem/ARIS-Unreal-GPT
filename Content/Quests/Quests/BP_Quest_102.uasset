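; Quest 102 logic: completes once the player has collected at least one artifact and one mineral, in either order.
; On BeginPlay it binds to the GameInstance's artifact and mineral collection events, each handler checking both collected arrays through count-check macros.
; When both are present, ARIS speaks a scripted German praise-and-return line and the quest log completes the quest.
; Otherwise a scripted ARIS line and debug print play, with only the mineral-first path updating the HUD objective.
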(event Custom|OnArtifactCollected
  (|MoreArtifactsThan
    (:true
      (|MoreMineralsThan_2
        (:true
          (Default|ProcessDialogue (.AC_AIBrain (CallFunction|GetDirectARIS)) true "Gut gemacht Operator. Komm vorerst zurück.")
          (Default|CompleteQuest (CallFunction|GetDirectQuestLogComponent) (.RowName (Utilities|Struct|BreakDataTableRowHandle (Variables|Default|GetQuestData)))))
        (:false
          (Development|PrintString "Collect a Mineral!")
          (CallFunction|PlayScriptedARIS "AfterTwoArtifacts"))))))

(event Custom|OnMineralCollected
  (|MoreMineralsThan
    (:true
      (|MoreArtifactsThan_2
        (:true
          (Default|ProcessDialogue (.AC_AIBrain (CallFunction|GetDirectARIS)) true "Gut gemacht Operator. Komm vorerst zurück.")
          (Default|CompleteQuest (CallFunction|GetDirectQuestLogComponent) (.RowName (Utilities|Struct|BreakDataTableRowHandle (Variables|Default|GetQuestData)))))
        (:false
          (Development|PrintString "Collect an Artifact")
          (Variables|/Script/UMG.TextBlock|SetText (Variables|/Game/UserInterface/HUD/UIPlayerHUD.UIPlayerHUD_C|GetMainQuestInfo (CallFunction|GetDirectHUDInterface)) "Finde ein Artefakt")
          (CallFunction|PlayScriptedARIS "AfterFirstCollect"))))))

(event EventBeginPlay
  (bind _asgame_instance_fp (CallFunction|GetDirectGameInstance))
  (EventDispatchers|BindEventtoOnArtifactCollected _asgame_instance_fp (delegate Custom|OnArtifactCollected))
  (EventDispatchers|BindEventtoOnMineralCollected _asgame_instance_fp (delegate Custom|OnMineralCollected)))

(fn ConstructionScript
  (|CallParentFunction))