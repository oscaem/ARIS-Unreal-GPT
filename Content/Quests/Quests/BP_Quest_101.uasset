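; Quest 101 Blueprint that completes when the game changes to a specific level, apparently after the first warp.
; BeginPlay binds Completed to the game instance's level-change event without calling the parent BeginPlay.
; On the matching level, ARIS's AI brain receives a scripted German request to find and describe colorful mineral veins, then the quest log completes the quest.
; An older timed PlayScriptedARIS sequence remains disconnected.
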(event Custom|Completed
  (params (ToLevel :type Level%20Enum :default "NewEnumerator0"))
  (if (Utilities|Enum|Equal(Enum) ToLevel "NewEnumerator1")
    (Default|ProcessDialogue (.AC_AIBrain (CallFunction|GetDirectARIS)) true "Es hat geklappt. Jetzt macht euch schnell auf die Suche nach Mineralvorkommen auf der Oberfläche. Sie Unterscheiden sich vom Gestein durch ihre Auffälligen Farben. Wenn ihr eine Ader gefunden habt, beschreibt sie mir.")
    (Default|CompleteQuest (CallFunction|GetDirectQuestLogComponent) (.RowName (Utilities|Struct|BreakDataTableRowHandle (Variables|Default|GetQuestData))))))

(event EventBeginPlay
  (EventDispatchers|BindEventtoOnLevelChanged (CallFunction|GetDirectGameInstance) (delegate Custom|Completed)))

(fn ConstructionScript
  (|CallParentFunction))