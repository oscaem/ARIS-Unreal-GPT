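; ARIS robot NPC actor that floats and turns to face the player while its look-at lock is on.
; BeginPlay applies one dynamic emissive material, shared with the AI brain component, to the robot meshes and starts a timeline-driven bob.
; AnimationLock toggles brain mode and tracking.
; Level-change setup only unbinds its handler, disabled-SOLA dialogue is left unwired, and TriggerAction only prints.
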(event EventBeginPlay
  (|CallParentFunction)
  (CallFunction|CreateMaterial)
  (|InitializeCallbacks)
  (|PlayFloatingAnimation))

(event EventTick
  (params (DeltaSeconds :type Float%20%28single-precision%29))
  (|CallParentFunction DeltaSeconds)
  (|TrackPlayer))

(fn ConstructionScript
  (|CallParentFunction))

(fn TriggerAction
  (params (Action :type ENPCAction%20Enum :default "NewEnumerator0"))
  (Development|PrintString "Triggering Action"))

(fn CreateMaterial
  (bind _robot (Variables|Default|Getrobot))
  (bind _returnvalue (Rendering|Material|CreateDynamicMaterialInstance _robot 0 "/Game/Actors/NPCs/Materials/ARIS/Materials/MI_EmissiveARIS.MI_EmissiveARIS" "None" :!class /Script/Engine.PrimitiveComponent))
  (bind _output_get (Variables|/Game/Core/Components/AC_AIBrain.AC_AIBrain_C|SetResponseMaterial (Variables|Default|GetAC_AIBrain) _returnvalue))
  (Rendering|Material|SetMaterial _robot 0 _output_get))

(fn AnimationLock
  (params (Start :type Boolean))
  (if Start
    (Default|SwitchMode (Variables|Default|GetAC_AIBrain) "NewEnumerator2")
    (Variables|Default|SetlocksOn false)
    (else
      (Default|SwitchMode (Variables|Default|GetAC_AIBrain) "NewEnumerator0")
      (Variables|Default|SetlocksOn true))))

(fn ToggleVisibility
  (params (Visible :type Boolean))
  (if Visible
    (Rendering|SetActorHiddenInGame false)
    (else
      (Rendering|SetActorHiddenInGame true))))

(event Custom|OnTalkedToDisabledSola
  (bind _returnvalue (Utilities|GetDataTableRow "/Game/Sound/Actors/ARIS/EArisVoicelineData.EArisVoicelineData" "DisabledSola")))

(event Custom|OnLevelChanged
  (params (ToLevel :type Level%20Enum :default "NewEnumerator0"))
  (if (Utilities|Enum|Equal(Enum) ToLevel "NewEnumerator2")
    (EventDispatchers|BindEventtoOnTalkedtoDisabledSola (.As%20SOLA (CallFunction|GetDirectSOLA)) (delegate Custom|OnTalkedToDisabledSola))))