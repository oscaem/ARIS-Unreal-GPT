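; BP_WarpGate is a warp platform that reveals destination portals while the first-person character stands inside its trigger.
; Overlap begin and end set a player-on-platform flag and toggle visibility on the first Glacier and Desert portal actors found in the level.
; Glacier shows its portal cylinder if unlocked in the game instance, otherwise its "Gesperrt" (locked) component.
; The Interaction event is empty, leaving the WarpToDesert call unreachable.
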(event OnComponentBeginOverlap(Trigger)
  (params (OverlappedComponent :type Primitive%20Component%20Object%20Reference) (OtherActor :type Actor%20Object%20Reference) (OtherComp :type Primitive%20Component%20Object%20Reference) (OtherBodyIndex :type Integer) (bFromSweep :type Boolean) (SweepResult :type Hit%20Result%20Structure%20%28by%20ref%29))
  ;[1 1 1] Enable Warp
  (Utilities|Casting|CastToBP_FirstPersonCharacter OtherActor)
  (Variables|Default|SetPlayerOnPlatform true)
  (CallFunction|SetPortalVisibility true))

(event OnComponentEndOverlap(Trigger)
  (params (OverlappedComponent :type Primitive%20Component%20Object%20Reference) (OtherActor :type Actor%20Object%20Reference) (OtherComp :type Primitive%20Component%20Object%20Reference) (OtherBodyIndex :type Integer))
  ;[1 1 1] Enable Warp
  (Utilities|Casting|CastToBP_FirstPersonCharacter OtherActor)
  (Variables|Default|SetPlayerOnPlatform false)
  (CallFunction|SetPortalVisibility false))

(event EventBeginPlay)

(event Collision|EventActorBeginOverlap
  (params (OtherActor :type Actor%20Object%20Reference)))

(event EventTick
  (params (DeltaSeconds :type Float%20%28single-precision%29)))

(event EventInteraction)

(fn ConstructionScript)

(fn SetPortalVisibility
  (params (bNewVisibility :type Boolean))
  (bind _outactors (Actor|GetAllActorsOfClass "/Game/Actors/Other/Ship/Warp/BP_Portal_Glacier.BP_Portal_Glacier_C"))
  (if (Variables|/Game/Core/GameInstanceFP.GameInstanceFP_C|GetGlacierUnlocked (CallFunction|GetDirectGameInstance))
    (Rendering|SetVisibility (Variables|/Game/Actors/Other/Ship/Warp/BP_Portal.BP_Portal_C|GetCylinder (Utilities|Array|Get(acopy) _outactors)) bNewVisibility true)
    (else
      (Rendering|SetVisibility (Variables|/Game/Actors/Other/Ship/Warp/BP_Portal_Glacier.BP_Portal_Glacier_C|GetGesperrt (Utilities|Array|Get(acopy) _outactors)) bNewVisibility true)))
  (bind _outactors_2 (Actor|GetAllActorsOfClass "/Game/Actors/Other/Ship/Warp/BP_Portal_Desert.BP_Portal_Desert_C"))
  (Rendering|SetVisibility (Variables|/Game/Actors/Other/Ship/Warp/BP_Portal.BP_Portal_C|GetCylinder (Utilities|Array|Get(acopy) _outactors_2)) bNewVisibility true)
  (return))