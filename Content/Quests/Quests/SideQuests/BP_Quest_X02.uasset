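; Side quest X02 Blueprint that resolves when SOLA hands over a material, logged as Trinite.
; On BeginPlay it binds to SOLA's OnMaterialGiven event, which writes the mineral into the collected list and broadcasts its collection.
; If SOLA accompanies, it flags her retrieved, dissolves her body and plays timed ARIS lines; otherwise it plays one line.
; Both branches complete the quest; the tenth artifact unveil is only a debug print.
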(event Custom|OnMaterialGiven
  (params (doesAccompany :type Boolean))
  (bind _asgame_instance_fp (CallFunction|GetDirectGameInstance))
  (bind _collectedminerals (Variables|/Game/Core/GameInstanceFP.GameInstanceFP_C|GetCollectedMinerals _asgame_instance_fp))
  (if (<= (Utilities|Array|Length _collectedminerals) 2)
    (Utilities|Array|Add _collectedminerals "NewEnumerator1")
    (else
      (Utilities|Array|SetArrayElem _collectedminerals 2 "NewEnumerator1")))
  (Development|PrintString "Adding Trinite To Inventory")
  (Default|CallOnMineralCollected (CallFunction|GetDirectGameInstance))
  (if doesAccompany
    (Variables|/Game/Core/GameInstanceFP.GameInstanceFP_C|SetSolaRetreived (CallFunction|GetDirectGameInstance) true)
    (Default|DissolveBody (.As%20SOLA (CallFunction|GetDirectSOLA)))
    (CallFunction|PlayScriptedARIS "AfterSolaCollect")
    (Utilities|FlowControl|Delay 4.0)
    (CallFunction|PlayScriptedARIS "AfterSolaCollect2")
    (Utilities|FlowControl|Delay 6.0)
    (CallFunction|PlayScriptedARIS "AfterSolaCollect3")
    (Utilities|FlowControl|Delay 1.0)
    (else
      (CallFunction|PlayScriptedARIS "AfterTalkSola")))
  (Development|PrintString "Unveil 10th Artifact")
  (Default|CompleteQuest (CallFunction|GetDirectQuestLogComponent) (Variables|Default|GetQuestID)))

(event EventBeginPlay
  (EventDispatchers|BindEventtoOnMaterialGiven (.As%20SOLA (CallFunction|GetDirectSOLA)) (delegate Custom|OnMaterialGiven)))

(fn ConstructionScript
  (|CallParentFunction))