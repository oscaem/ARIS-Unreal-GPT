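; Quest 103 Blueprint that unlocks the Glacier area when the player warps to a specific level.
; It binds to the game instance's warp and cutscene-ended events, then on that warp sets the GlacierUnlocked flag and reveals the Glacier portal.
; It then plays the ARIS "AfterFirstAct" script and the unlock sequence, completing the quest when that cutscene ends.
; Parent BeginPlay is not executed.
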(event Custom|Completed
  (params (ToLevel :type Level%20Enum :default "NewEnumerator0"))
  (if (Utilities|Enum|Equal(Enum) ToLevel "NewEnumerator0")
    (Variables|/Game/Core/GameInstanceFP.GameInstanceFP_C|SetGlacierUnlocked (CallFunction|GetDirectGameInstance) true)
    (|enableportal
      (:NewParam2
        (Development|PrintString "Play Glacier Cutscene")
        (CallFunction|PlayScriptedARIS "AfterFirstAct")
        (Default|PlaySequence (CallFunction|GetDirectGameInstance) "/Game/Movies/Cin_GlacierUnlocked.Cin_GlacierUnlocked")))))

(event Custom|OnCutsceneEnded
  (params (PlayedCutscene :type Level%20Sequence%20Actor%20Object%20Reference))
  (if (== (Class|LevelSequenceActor|GetSequence PlayedCutscene) "/Game/Movies/Cin_GlacierUnlocked.Cin_GlacierUnlocked")
    (Default|CompleteQuest (CallFunction|GetDirectQuestLogComponent) (.RowName (Utilities|Struct|BreakDataTableRowHandle (Variables|Default|GetQuestData))))))

(event EventBeginPlay
  (bind _asgame_instance_fp (CallFunction|GetDirectGameInstance))
  (EventDispatchers|BindEventtoOnPlayerWarped _asgame_instance_fp (delegate Custom|Completed))
  (EventDispatchers|BindEventtoOnCutsceneEnded _asgame_instance_fp (delegate Custom|OnCutsceneEnded)))

(fn ConstructionScript
  (|CallParentFunction))