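; Side quest Blueprint X01, which tracks artifact collection and completes the quest at ten artifacts.
; On BeginPlay it binds to the game instance's artifact-collected event, leaving the parent BeginPlay call unconnected.
; Each event checks the collected count: the third artifact only prints a "ENABLE SOLA" placeholder, and the tenth completes the quest through the quest log component.
; The count function's array-length lookup appears unconnected.
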(event Custom|OnArtifactCollected
  (bind _artifacts (|HowManyArtifactsCollected?))
  (if (== _artifacts 3)
    (Development|PrintString "ENABLE SOLA")
    (elif (== _artifacts 10)
      (Default|CompleteQuest (CallFunction|GetDirectQuestLogComponent) (Variables|Default|GetQuestID)))))

(event EventBeginPlay
  (EventDispatchers|BindEventtoOnArtifactCollected (CallFunction|GetDirectGameInstance) (delegate Custom|OnArtifactCollected)))

(fn ConstructionScript
  (|CallParentFunction))