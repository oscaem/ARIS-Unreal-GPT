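; BP_Mineral_TriniteDummy is a dummy Trinite mineral actor that triggers a scripted voice or dialogue reaction when interacted with.
; Its Box1 overlap registers it as the first-person character's current interactable, sets Scannable and shows a "SCANNEN" HUD prompt, clearing all three on exit.
; Interaction sends a fixed German hands-off line to SOLA's ACAIBrain if SOLA is enabled; otherwise it prints a debug string and plays scripted ARIS "Trinit".
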(event OnComponentBeginOverlap(Box1)
  (params (OverlappedComponent :type Primitive%20Component%20Object%20Reference) (OtherActor :type Actor%20Object%20Reference) (OtherComp :type Primitive%20Component%20Object%20Reference) (OtherBodyIndex :type Integer) (bFromSweep :type Boolean) (SweepResult :type Hit%20Result%20Structure%20%28by%20ref%29))
  (bind _asbp_first_person_character (Utilities|Casting|CastToBP_FirstPersonCharacter OtherActor))
  (Variables|/Game/Actors/Player/BP_FirstPersonCharacter.BP_FirstPersonCharacter_C|SetCurrentInteractable _asbp_first_person_character self)
  (Variables|Default|SetScannable true)
  (Default|DisplayActionPrompt (CallFunction|GetDirectHUDInterface) "SCANNEN" true))

(event OnComponentEndOverlap(Box1)
  (params (OverlappedComponent :type Primitive%20Component%20Object%20Reference) (OtherActor :type Actor%20Object%20Reference) (OtherComp :type Primitive%20Component%20Object%20Reference) (OtherBodyIndex :type Integer))
  (bind _asbp_first_person_character (Utilities|Casting|CastToBP_FirstPersonCharacter OtherActor))
  (Variables|/Game/Actors/Player/BP_FirstPersonCharacter.BP_FirstPersonCharacter_C|SetCurrentInteractable _asbp_first_person_character 0)
  (Variables|Default|SetScannable false)
  (Default|DisplayActionPrompt (CallFunction|GetDirectHUDInterface) "" false))

(event EventInteraction
  (if (Variables|/Game/Core/GameInstanceFP.GameInstanceFP_C|GetSolaEnabled (CallFunction|GetDirectGameInstance))
    (Default|ProcessDialogue (Variables|/Game/Actors/NPCs/BP_NPC_SOLA.BP_NPC_SOLA_C|GetAC_AIBrain (.As%20SOLA (CallFunction|GetDirectSOLA))) true "Finger weg von meinen Mineralien!")
    (else
      (Development|PrintString "Weird")
      (CallFunction|PlayScriptedARIS "Trinit"))))

(fn ConstructionScript)