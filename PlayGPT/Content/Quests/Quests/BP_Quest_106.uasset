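; Quest 106 Blueprint that completes once more than one mineral is collected, branching ARIS's reaction on artifact progress.
; It binds to the GameInstance's mineral-collected event and checks collection counts through two threshold macros.
; With more than two artifacts ARIS plays the AfterThirdCollect script; otherwise it speaks robot noise, is muted and "Bad Ending" prints.
; The parent BeginPlay is not called.
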(event Custom|OnMineralCollected
  (bind _ac_aibrain (CallFunction|GetDirectARIS))
  (|MoreMineralsThan_2_2 1
    (:true
      (|MoreArtifactsThan_2_2_2 2
        (:true
          (CallFunction|PlayScriptedARIS "AfterThirdCollect")
          (Development|PrintString "Found 3rd Mineral"))
        (:false
          (Default|Speak _ac_aibrain "/Game/Sound/Actors/SOLA/robot-noise.robot-noise" "NewEnumerator5")
          (Variables|/Game/Core/Components/AC_AIBrain.AC_AIBrain_C|SetisAllowedToTalk _ac_aibrain false)
          (Development|PrintString "Bad Ending")))
      (Default|CompleteQuest (CallFunction|GetDirectQuestLogComponent) (.RowName (Utilities|Struct|BreakDataTableRowHandle (Variables|Default|GetQuestData)))))))

(event EventBeginPlay
  (EventDispatchers|BindEventtoOnMineralCollected (CallFunction|GetDirectGameInstance) (delegate Custom|OnMineralCollected)))

(fn ConstructionScript
  (|CallParentFunction))