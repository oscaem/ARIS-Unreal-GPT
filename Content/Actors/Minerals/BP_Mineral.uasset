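; A scannable mineral pickup that the first-person character collects as a sample, removing itself on BeginPlay if already collected.
; Overlapping its box registers it as the character's current interactable and shows a scan prompt.
; Interaction, while fewer than three minerals are collected, records the sample in the game instance and plays a scan sound.
; A timeline then drives a dynamic material's Appearance parameter to dissolve the mesh before destroying the actor.
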(event OnComponentBeginOverlap(Box)
  (params (OverlappedComponent :type Primitive%20Component%20Object%20Reference) (OtherActor :type Actor%20Object%20Reference) (OtherComp :type Primitive%20Component%20Object%20Reference) (OtherBodyIndex :type Integer) (bFromSweep :type Boolean) (SweepResult :type Hit%20Result%20Structure%20%28by%20ref%29))
  ;[1 1 1] Enable Scanning
  (bind _asbp_first_person_character (Utilities|Casting|CastToBP_FirstPersonCharacter OtherActor))
  (Variables|/Game/Actors/Player/BP_FirstPersonCharacter.BP_FirstPersonCharacter_C|SetCurrentInteractable _asbp_first_person_character self)
  (Variables|Default|SetScannable true)
  (Default|DisplayActionPrompt (CallFunction|GetDirectHUDInterface) "SCANNEN" true))

(event OnComponentEndOverlap(Box)
  (params (OverlappedComponent :type Primitive%20Component%20Object%20Reference) (OtherActor :type Actor%20Object%20Reference) (OtherComp :type Primitive%20Component%20Object%20Reference) (OtherBodyIndex :type Integer))
  ;[1 1 1] Enable Scanning
  (bind _asbp_first_person_character (Utilities|Casting|CastToBP_FirstPersonCharacter OtherActor))
  (Variables|/Game/Actors/Player/BP_FirstPersonCharacter.BP_FirstPersonCharacter_C|SetCurrentInteractable _asbp_first_person_character 0)
  (Variables|Default|SetScannable false)
  (Default|DisplayActionPrompt (CallFunction|GetDirectHUDInterface) "" false))

(event Custom|Dissolve
  (bind _cube (Variables|Default|GetCube))
  ;[1 1 1] Dissolve
  (bind _returnvalue (Rendering|Material|CreateDynamicMaterialInstance (Rendering|Material|GetMaterial _cube 0) "None" "None" :!class /Script/Engine.KismetMaterialLibrary))
  (bind _output_get (Variables|Default|SetDynamicMaterialInstance _returnvalue))
  (Rendering|Material|SetMaterial _cube 0 _output_get)
  (Audio|PlaySound2D "/Game/Sound/Effects/Actions/Effect_Scan.Effect_Scan" 1.0 1.0 0.0 0 0)
  (bind _dissolveamount (Timeline|DissolveTimeline Play)
    (:Update
      (Rendering|Material|SetScalarParameterValue _output_get "Appearance" _dissolveamount :!class /Script/Engine.MaterialInstanceDynamic))
    (:Finished
      (Actor|DestroyActor))))

(event EventBeginPlay
  (if (Utilities|Array|ContainsItem (Variables|/Game/Core/GameInstanceFP.GameInstanceFP_C|GetCollectedMinerals (CallFunction|GetDirectGameInstance)) (Variables|Default|GetMineral))
    (Actor|DestroyActor)))

(event Collision|EventActorBeginOverlap
  (params (OtherActor :type Actor%20Object%20Reference)))

(event EventTick
  (params (DeltaSeconds :type Float%20%28single-precision%29)))

(event EventInteraction
  ;[1 1 1] Interact
  (if (Variables|Default|GetScannable)
    (bind _asgame_instance_fp (Utilities|Casting|CastToGameInstanceFP (Game|GetGameInstance)))
    (if (<= (Utilities|Array|Length (Variables|/Game/Core/GameInstanceFP.GameInstanceFP_C|GetCollectedMinerals _asgame_instance_fp)) 2)
      (Variables|Default|SetScannable false)
      (Development|PrintString "Scanning")
      (CallFunction|Dissolve)
      (Default|ScanMineralSample _asgame_instance_fp (Variables|Default|GetMineral))
      (Development|PrintString "Hello")
      (else
        (Development|PrintString "Already Collected Three Minerals")))
    (else
      (Development|PrintString "Can't Scan"))))

(fn ConstructionScript)