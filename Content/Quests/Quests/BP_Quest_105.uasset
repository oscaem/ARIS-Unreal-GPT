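; Quest 105 Blueprint that completes when enough minerals are collected and decides whether ARIS remains stable.
; On BeginPlay it binds to the game instance's mineral-collected event, then checks whether the collected mineral count exceeds one.
; If so, the artifact count either reports ARIS stable or clears its stability flag on the game instance.
; Either outcome plays the scripted "AfterSecondAct" ARIS sequence and completes the quest through the quest log component.
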(event Custom|OnMineralCollected
  (|MoreMineralsThan_2 1
    (:true
      (|MoreArtifactsThan_2_2 4
        (:true
          (Development|PrintString "ARIS Is Stable"))
        (:false
          (Development|PrintString "ARIS Is getting Unstable")
          (Variables|/Game/Core/GameInstanceFP.GameInstanceFP_C|SetARISstable (CallFunction|GetDirectGameInstance) false)))
      (CallFunction|PlayScriptedARIS "AfterSecondAct")
      (Default|CompleteQuest (CallFunction|GetDirectQuestLogComponent) (.RowName (Utilities|Struct|BreakDataTableRowHandle (Variables|Default|GetQuestData)))))))

(event EventBeginPlay
  (EventDispatchers|BindEventtoOnMineralCollected (CallFunction|GetDirectGameInstance) (delegate Custom|OnMineralCollected)))

(fn ConstructionScript
  (|CallParentFunction))