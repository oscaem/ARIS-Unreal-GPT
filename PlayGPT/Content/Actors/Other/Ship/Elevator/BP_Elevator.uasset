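; Ship elevator that teleports the player between two floors, the bridge (top) and storage (bottom).
; Top and Bottom overlaps register it as the first-person character's CurrentInteractable and show the destination's German name as a HUD prompt, clearing both on exit.
; Interaction moves the player to the first BP_FloorPivotBottom or BP_FloorPivotTop found, sets a fixed rotation and flips IsTop.
; The destination follows that flag rather than the overlapped trigger.
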(event OnComponentBeginOverlap(Top)
  (params (OverlappedComponent :type Primitive%20Component%20Object%20Reference) (OtherActor :type Actor%20Object%20Reference) (OtherComp :type Primitive%20Component%20Object%20Reference) (OtherBodyIndex :type Integer) (bFromSweep :type Boolean) (SweepResult :type Hit%20Result%20Structure%20%28by%20ref%29))
  (bind _asbp_first_person_character (Utilities|Casting|CastToBP_FirstPersonCharacter OtherActor))
  (Variables|/Game/Actors/Player/BP_FirstPersonCharacter.BP_FirstPersonCharacter_C|SetCurrentInteractable _asbp_first_person_character self)
  (bind _ashud (Utilities|Casting|CastToHUD (HUD|GetHUD (Game|GetPlayerController 0))))
  (Default|DisplayActionPrompt (Variables|/Game/UserInterface/HUD/HUD.HUD_C|GetPlayer%20HUD _ashud) "LAGER" true))

(event OnComponentEndOverlap(Top)
  (params (OverlappedComponent :type Primitive%20Component%20Object%20Reference) (OtherActor :type Actor%20Object%20Reference) (OtherComp :type Primitive%20Component%20Object%20Reference) (OtherBodyIndex :type Integer))
  (bind _asbp_first_person_character (Utilities|Casting|CastToBP_FirstPersonCharacter OtherActor))
  (Variables|/Game/Actors/Player/BP_FirstPersonCharacter.BP_FirstPersonCharacter_C|SetCurrentInteractable _asbp_first_person_character 0)
  (bind _ashud (Utilities|Casting|CastToHUD (HUD|GetHUD (Game|GetPlayerController 0))))
  (Default|DisplayActionPrompt (Variables|/Game/UserInterface/HUD/HUD.HUD_C|GetPlayer%20HUD _ashud) "" false))

(event OnComponentBeginOverlap(Bottom)
  (params (OverlappedComponent :type Primitive%20Component%20Object%20Reference) (OtherActor :type Actor%20Object%20Reference) (OtherComp :type Primitive%20Component%20Object%20Reference) (OtherBodyIndex :type Integer) (bFromSweep :type Boolean) (SweepResult :type Hit%20Result%20Structure%20%28by%20ref%29))
  (bind _asbp_first_person_character (Utilities|Casting|CastToBP_FirstPersonCharacter OtherActor))
  (Variables|/Game/Actors/Player/BP_FirstPersonCharacter.BP_FirstPersonCharacter_C|SetCurrentInteractable _asbp_first_person_character self)
  (bind _ashud (Utilities|Casting|CastToHUD (HUD|GetHUD (Game|GetPlayerController 0))))
  (Default|DisplayActionPrompt (Variables|/Game/UserInterface/HUD/HUD.HUD_C|GetPlayer%20HUD _ashud) "BRÜCKE" true))

(event OnComponentEndOverlap(Bottom)
  (params (OverlappedComponent :type Primitive%20Component%20Object%20Reference) (OtherActor :type Actor%20Object%20Reference) (OtherComp :type Primitive%20Component%20Object%20Reference) (OtherBodyIndex :type Integer))
  (bind _asbp_first_person_character (Utilities|Casting|CastToBP_FirstPersonCharacter OtherActor))
  (Variables|/Game/Actors/Player/BP_FirstPersonCharacter.BP_FirstPersonCharacter_C|SetCurrentInteractable _asbp_first_person_character 0)
  (bind _ashud (Utilities|Casting|CastToHUD (HUD|GetHUD (Game|GetPlayerController 0))))
  (Default|DisplayActionPrompt (Variables|/Game/UserInterface/HUD/HUD.HUD_C|GetPlayer%20HUD _ashud) "" false))

(event EventBeginPlay)

(event Collision|EventActorBeginOverlap
  (params (OtherActor :type Actor%20Object%20Reference)))

(event EventTick
  (params (DeltaSeconds :type Float%20%28single-precision%29)))

(event EventInteraction
  (bind _returnvalue (Game|GetPlayerCharacter 0))
  (bind _returnvalue_2 (Game|GetPlayerCharacter 0))
  (if (Variables|Default|GetisTop)
    (bind _outactors (Actor|GetAllActorsOfClass "/Game/Actors/Other/Ship/Elevator/BP_FloorPivotBottom.BP_FloorPivotBottom_C"))
    (Transformation|SetActorLocation _returnvalue_2 (Transformation|GetActorLocation (Utilities|Array|Get(acopy) _outactors)) false true)
    (Transformation|SetActorRotation _returnvalue_2 "0.000000,-60.000000,0.000000")
    (Variables|Default|SetisTop false)
    (else
      (bind _outactors_2 (Actor|GetAllActorsOfClass "/Game/Actors/Other/Ship/Elevator/BP_FloorPivotTop.BP_FloorPivotTop_C"))
      (Transformation|SetActorLocation _returnvalue (Transformation|GetActorLocation (Utilities|Array|Get(acopy) _outactors_2)) false true)
      (Transformation|SetActorRotation _returnvalue "0.000000,-60.000000,0.000000")
      (Variables|Default|SetisTop true))))

(fn ConstructionScript)