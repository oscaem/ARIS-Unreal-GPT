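; SOLA NPC actor, a robot that reacts to the player's approach and interaction depending on whether it is enabled.
; Its trigger box sets the current interactable and game instance state, then plays scripted ARIS dialogue or shows an analyse prompt.
; Interacting while disabled plays a noise and fires a delayed event, while AI actions raise material-given events.
; Dynamic materials drive the AI response glow and a timeline dissolve, which ends in ARIS dialogue and destruction.
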(event OnComponentBeginOverlap(Box1)
  (params (OverlappedComponent :type Primitive%20Component%20Object%20Reference) (OtherActor :type Actor%20Object%20Reference) (OtherComp :type Primitive%20Component%20Object%20Reference) (OtherBodyIndex :type Integer) (bFromSweep :type Boolean) (SweepResult :type Hit%20Result%20Structure%20%28by%20ref%29))
  (bind _asgame_instance_fp (CallFunction|GetDirectGameInstance))
  (bind _asbp_first_person_character (Utilities|Casting|CastToBP_FirstPersonCharacter OtherActor))
  (Variables|/Game/Actors/Player/BP_FirstPersonCharacter.BP_FirstPersonCharacter_C|SetCurrentInteractable _asbp_first_person_character self)
  (Variables|/Game/Core/GameInstanceFP.GameInstanceFP_C|SetConnectedNPC (CallFunction|GetDirectGameInstance) "NewEnumerator1")
  (Variables|/Game/Core/GameInstanceFP.GameInstanceFP_C|SetatSola _asgame_instance_fp true)
  (Development|PrintString "At Soa")
  (bind _ashud (Utilities|Casting|CastToHUD (HUD|GetHUD (Game|GetPlayerController 0))))
  (if (Variables|/Game/Core/GameInstanceFP.GameInstanceFP_C|GetSolaEnabled _asgame_instance_fp)
    (Default|ProcessDialogue (.AC_AIBrain (CallFunction|GetDirectARIS)) true "Eine Maschine? Schalte auf Übersetzungsmodus.")
    (else
      (Default|DisplayActionPrompt (Variables|/Game/UserInterface/HUD/HUD.HUD_C|GetPlayer%20HUD _ashud) "ANALYSIEREN" true))))

(event OnComponentEndOverlap(Box1)
  (params (OverlappedComponent :type Primitive%20Component%20Object%20Reference) (OtherActor :type Actor%20Object%20Reference) (OtherComp :type Primitive%20Component%20Object%20Reference) (OtherBodyIndex :type Integer))
  (bind _asbp_first_person_character (Utilities|Casting|CastToBP_FirstPersonCharacter OtherActor))
  (Variables|/Game/Actors/Player/BP_FirstPersonCharacter.BP_FirstPersonCharacter_C|SetCurrentInteractable _asbp_first_person_character 0)
  (Variables|/Game/Core/GameInstanceFP.GameInstanceFP_C|SetConnectedNPC (CallFunction|GetDirectGameInstance) "NewEnumerator0")
  (bind _ashud (Utilities|Casting|CastToHUD (HUD|GetHUD (Game|GetPlayerController 0))))
  (Variables|/Game/Core/GameInstanceFP.GameInstanceFP_C|SetatSola (CallFunction|GetDirectGameInstance) false))

(event Custom|DissolveBody
  (bind _returnvalue (Rendering|Material|CreateDynamicMaterialInstance (Rendering|Material|GetMaterial (Variables|Default|GetStaticMesh) 0) "None" "None" :!class /Script/Engine.KismetMaterialLibrary))
  (bind _output_get (Variables|Default|SetDynamicMaterialInstance _returnvalue))
  (Rendering|Material|SetMaterial (Variables|Default|GetStaticMesh) 0 _output_get)
  (Audio|PlaySound2D "/Game/Sound/Effects/Actions/Effect_Scan.Effect_Scan" 1.0 1.0 0.0 0 0)
  (bind _dissolveamount (Timeline|Timeline Play)
    (:Update
      (Rendering|Material|SetScalarParameterValue _output_get "Appearance" _dissolveamount :!class /Script/Engine.MaterialInstanceDynamic))
    (:Finished
      (Default|ProcessDialogue (.AC_AIBrain (CallFunction|GetDirectARIS)) true "Oh, Hallo, wer bist du denn? Ein Freund?")
      (Actor|DestroyActor))))

(event EventBeginPlay
  (CallFunction|CreateMaterial))

(event Collision|EventActorBeginOverlap
  (params (OtherActor :type Actor%20Object%20Reference)))

(event EventTick
  (params (DeltaSeconds :type Float%20%28single-precision%29)))

(event EventInteraction
  (if (Variables|/Game/Core/GameInstanceFP.GameInstanceFP_C|GetSolaEnabled (CallFunction|GetDirectGameInstance))
    (Development|PrintString "Talking To Sola")
    (else
      (Development|PrintString "Sola Disabled")
      (Audio|PlaySound2D "/Game/Sound/Actors/SOLA/robot-noise.robot-noise" 3.0 1.0 0.0 0 0)
      (Utilities|FlowControl|Delay 3.0)
      (Default|CallOnTalkedtoDisabledSola))))

(fn ConstructionScript
  (|CallParentFunction))

(fn CreateMaterial
  (bind _returnvalue (Rendering|Material|CreateDynamicMaterialInstance (Variables|Default|GetStaticMesh) 1 "/Game/Actors/NPCs/Materials/ARIS/Materials/MI_EmissiveARIS.MI_EmissiveARIS" "None" :!class /Script/Engine.PrimitiveComponent))
  (bind _output_get (Variables|/Game/Core/Components/AC_AIBrain.AC_AIBrain_C|SetResponseMaterial (Variables|Default|GetAC_AIBrain) _returnvalue))
  (Rendering|Material|SetMaterial (Variables|Default|GetStaticMesh) 1 _output_get))

(fn TriggerAction
  (params (Action :type ENPCAction%20Enum :default "NewEnumerator0"))
  (switch Utilities|FlowControl|Switch|SwitchonENPCAction Action
    (:NewEnumerator2
      (Default|CallOnMaterialGiven false))
    (:NewEnumerator3
      (Default|CallOnMaterialGiven true))))