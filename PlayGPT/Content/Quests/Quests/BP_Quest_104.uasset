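; Quest 104 Blueprint that completes when the player warps to a specific level, apparently the glacier.
; On BeginPlay it binds to the game instance's player-warped event.
; When the destination matches the target enum entry, it plays the "AfterWarpGlacier" scripted ARIS line and completes the quest in the quest log by its data row name.
; The parent BeginPlay call is left disconnected.
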(event Custom|Completed
  (params (ToLevel :type Level%20Enum :default "NewEnumerator0"))
  (if (Utilities|Enum|Equal(Enum) ToLevel "NewEnumerator2")
    (CallFunction|PlayScriptedARIS "AfterWarpGlacier")
    (Default|CompleteQuest (CallFunction|GetDirectQuestLogComponent) (.RowName (Utilities|Struct|BreakDataTableRowHandle (Variables|Default|GetQuestData))))))

(event EventBeginPlay
  (EventDispatchers|BindEventtoOnPlayerWarped (CallFunction|GetDirectGameInstance) (delegate Custom|Completed)))

(fn ConstructionScript
  (|CallParentFunction))