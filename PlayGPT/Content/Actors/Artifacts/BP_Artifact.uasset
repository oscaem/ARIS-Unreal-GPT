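; BP_Artifact is a collectible that the first-person character scans through an overlap-driven interaction prompt.
; On each game instance level change, it destroys itself if already collected, while one special artifact survives only once at least nine are collected.
; Interaction records the scan, shows a HUD badge, and runs a timeline-driven dynamic material dissolve.
; When the dissolve finishes, it sends its story to the ARIS AI brain as scripted dialogue and destroys itself.
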(event OnComponentBeginOverlap(Box)
  (params (OverlappedComponent :type Primitive%20Component%20Object%20Reference) (OtherActor :type Actor%20Object%20Reference) (OtherComp :type Primitive%20Component%20Object%20Reference) (OtherBodyIndex :type Integer) (bFromSweep :type Boolean) (SweepResult :type Hit%20Result%20Structure%20%28by%20ref%29))
  ;[1 1 1] HandleBounds
  (bind _asbp_first_person_character (Utilities|Casting|CastToBP_FirstPersonCharacter OtherActor))
  (Variables|/Game/Actors/Player/BP_FirstPersonCharacter.BP_FirstPersonCharacter_C|SetCurrentInteractable _asbp_first_person_character self)
  (Default|DisplayActionPrompt (CallFunction|GetDirectHUDInterface) "ANALYSIEREN" true))

(event OnComponentEndOverlap(Box)
  (params (OverlappedComponent :type Primitive%20Component%20Object%20Reference) (OtherActor :type Actor%20Object%20Reference) (OtherComp :type Primitive%20Component%20Object%20Reference) (OtherBodyIndex :type Integer))
  ;[1 1 1] HandleBounds
  (bind _asbp_first_person_character (Utilities|Casting|CastToBP_FirstPersonCharacter OtherActor))
  (Variables|/Game/Actors/Player/BP_FirstPersonCharacter.BP_FirstPersonCharacter_C|SetCurrentInteractable _asbp_first_person_character 0)
  (Default|DisplayActionPrompt (CallFunction|GetDirectHUDInterface) "" false))

(event Custom|Dissolve
  ;[1 1 1] DISSOLVE
  (CallFunction|PlayArtifactBadge)
  (|HandleDissolve
    (:Finished
      (CallFunction|PlayArtifactDialogue)
      (Actor|DestroyActor))))

(event Custom|CustomEvent
  (params (ToLevel :type Level%20Enum :default "NewEnumerator0"))
  (bind _self self)
  (bind _defaultsceneroot (Variables|Default|GetDefaultSceneRoot _self))
  (if (Utilities|Enum|Equal(Enum) (Variables|Default|GetArtifact) "NewEnumerator11")
    (if (>= (Utilities|Array|Length (Variables|/Game/Core/GameInstanceFP.GameInstanceFP_C|GetCollectedArtifacts (CallFunction|GetDirectGameInstance))) 9)
      (Rendering|SetVisibility _defaultsceneroot true false)
      (else
        (Rendering|SetVisibility _defaultsceneroot false false)
        (Actor|DestroyActor)))
    (elif (Utilities|Array|ContainsItem (Variables|/Game/Core/GameInstanceFP.GameInstanceFP_C|GetCollectedArtifacts (CallFunction|GetDirectGameInstance)) (Variables|Default|GetArtifact))
      (Rendering|SetVisibility (Variables|Default|GetDefaultSceneRoot self) false false)
      (Actor|DestroyActor)
      (else
        (Rendering|SetVisibility (Variables|Default|GetDefaultSceneRoot self) true false)))))

(event EventBeginPlay
  (EventDispatchers|BindEventtoOnLevelChanged (CallFunction|GetDirectGameInstance) (delegate Custom|CustomEvent)))

(event EventInteraction
  ;[1 1 1] INTERACT
  (Default|ScanArtifact (CallFunction|GetDirectGameInstance) (.Artifact (Utilities|Struct|BreakArtifactProperties (Variables|Default|GetArtifactProps))))
  (CallFunction|Dissolve))

(fn ConstructionScript)

(fn PlayArtifactBadge
  (bind _ashud (Utilities|Casting|CastToHUD (HUD|GetHUD (Game|GetPlayerController 0))))
  (Audio|PlaySound2D "/Game/Sound/Effects/UI/Effect_Achievement_Rare.Effect_Achievement_Rare" 0.8 1.0 0.0 0 0)
  (Default|DisplayArtifactBadge (Variables|/Game/UserInterface/HUD/HUD.HUD_C|GetPlayer%20HUD _ashud) (.Artifact (Utilities|Struct|BreakArtifactProperties (Variables|Default|GetArtifactProps)))))

(fn PlayArtifactDialogue
  (Default|ProcessDialogue (Variables|/Game/Actors/NPCs/BP_NPC_ARIS.BP_NPC_ARIS_C|GetAC_AIBrain (.ARIS (CallFunction|GetDirectARIS))) true (Utilities|String|ToString(Text) (.Story (Utilities|Struct|BreakArtifactProperties (Variables|Default|GetArtifactProps))))))